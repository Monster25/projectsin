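; Prototype enemy that damages the player character by periodic box trace and drops random loot when killed.
; Tick prints Health, then after a 2-second Delay runs a debug-drawn trace, offset by scaled actor location rather than forward vector, subtracting player health whatever the combat state.
; DealDamageToMe lowers Health; at zero, SpawnItem spawns an item with the ID resolved from a random LootTable row's data table reference, and the enemy is destroyed.
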(event `self.ReceiveBeginPlay`)

(event `self.ReceiveTick`
  (params (DeltaSeconds :type "Float (single-precision)"))
  (bind _returnvalue (`self.K2_GetActorLocation`))
  (`KismetSystemLibrary.PrintString` (`KismetStringLibrary.Conv_DoubleToString` (`self.Health`)) true true (struct :`G` 0.66 :`B` 1.0 :`A` 1.0) 0.0)
  (`KismetSystemLibrary.Delay` 2.0)
  (bind (_outhit _returnvalue_2) (`KismetSystemLibrary.BoxTraceSingleForObjects` :`Start` (`KismetMathLibrary.MakeVector` (.x _returnvalue) (.y _returnvalue) (+ (.z _returnvalue) 200.0)) :`End` (+ _returnvalue (* _returnvalue 300.0)) :`HalfSize` (25.0 25.0 25.0) :`Orientation` (`self.K2_GetActorRotation` self) :`ObjectTypes` (`|MakeArray` "ObjectTypeQuery3" "ObjectTypeQuery1" "ObjectTypeQuery2" :!type "EObjectTypeQuery Enum") :`DrawDebugType` "ForDuration" :`DrawTime` 2.0))
  (if _returnvalue_2
    (bind _asmy_character (cast `/Game/Blueprints/Player/MyCharacter` (`.HitActor` (`GameplayStatics.BreakHitResult` _outhit))))
    (bind _value (`/Game/Blueprints/Player/Components/CombatComponent.GetCurrentState` (`/Game/Blueprints/Player/MyCharacter.CombatComponent` _asmy_character)))
    (switch `/Game/Blueprints/Player/Components/E_CombatComponent_States` _value
      (:`NewEnumerator3`
        _)
      (:`NewEnumerator0`
        _)
      (:`NewEnumerator1`
        _)
      (:`NewEnumerator2`
        _))
    (bind _attributescomponent (`/Game/Blueprints/Player/MyCharacter.AttributesComponent` _asmy_character))
    (bind _health (`/Game/Blueprints/Player/Components/AttributesComponent.GetHealth` _attributescomponent))
    (`/Game/Blueprints/Player/Components/AttributesComponent.SetHealth` _attributescomponent (- _health 10.0))))

(fn `DealDamageToMe`
  (params (IncomingDamage :type "Float (double-precision)"))
  (bind _health (`self.Health`))
  (set `self.Health` (- _health IncomingDamage))
  (if (<= _health 0.0)
    (`self.SpawnItem`)
    (`self.K2_DestroyActor`)))

(fn `SpawnItem`
  (bind _outrownames (`DataTableFunctionLibrary.GetDataTableRowNames` (`self.LootTable`)))
  (bind _result (`/Engine/EditorBlueprintResources/StandardMacros.DecrementInt` (`KismetArrayLibrary.Array_Length` _outrownames))
    (:`  `
      (bind _returnvalue (`|SpawnActorFromClass` (`self.ItemSpawnClass`) (`KismetMathLibrary.Conv_VectorToTransform` (`self.K2_GetActorLocation`)) "Undefined" "OverrideRootScale" null null))
      (bind _returnvalue_2 (`|GetDataTableRow` (`self.LootTable`) (`|GetArrayItem` _outrownames (`KismetMathLibrary.RandomIntegerInRange` 0 _result)))
        (:`then`
          (bind (_datatable _rowname) (break `DataTableRowHandle` (`.ItemRef_2_29F2FD6546C5CB6F6622CE8DA0C13A1D` (break `/Game/GameData/Items/Structures/LootStructs/Struct_LootTableData` _returnvalue_2))))
          (bind _returnvalue_3 (`|GetDataTableRow` _datatable _rowname)
            (:`then`
              (`/Game/Blueprints/Pickups/BP_Item.SetItemId` _returnvalue (`.ID_11_05CB8AEF472481D61C5566A382762853` (break `/Game/GameData/Items/Structures/ItemStructs/Struct_ItemData` _returnvalue_3))))))))))

(fn `UserConstructionScript`)