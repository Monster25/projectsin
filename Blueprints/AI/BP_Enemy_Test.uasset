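; BP_Enemy_Test is a test enemy actor with a Health value that can be damaged and destroyed.
; TakeDamage passes the damage amount to DealDamageToMe, which subtracts it from Health.
; Tick polls Health each frame, destroying the actor at zero or below, and prints the current value to screen as a debug readout.
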(event `self.ReceiveTick`
  (params (DeltaSeconds :type "Float (single-precision)"))
  (`|ExecutionSequence`
    (:`then_0`
      (if (<= (`self.Health`) 0.0)
        (`self.K2_DestroyActor`)))
    (:`then_1`
      (`KismetSystemLibrary.PrintString` (`KismetStringLibrary.Conv_DoubleToString` (`self.Health`)) true true (struct :`G` 0.66 :`B` 1.0 :`A` 1.0) 0.0))))

(event `/Game/Blueprints/AI/Interfaces/BPI_Damageable.TakeDamage`
  (params (DamageAmount :type "Float (single-precision)"))
  (`self.DealDamageToMe` DamageAmount))

(fn `DealDamageToMe`
  (params (Damage :type "Float (double-precision)"))
  (set `self.Health` (- (`self.Health`) Damage)))

(fn `UserConstructionScript`)