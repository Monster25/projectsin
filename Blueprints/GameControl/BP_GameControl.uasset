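; Game control Blueprint that procedurally generates a maze-like level of rooms on a square grid at BeginPlay.
; A seeded random walk carves path and bridge cells inside the border, backtracking from dead ends until no bridges remain.
; It spawns path rooms, then marks unused cells as walls, optionally turning a random wall into a loop path.
; Border and wall rooms spawn only when their show flags are set.
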(event `self.ReceiveBeginPlay`
  ;[0.8036 0.6791 1] Generate the Level
  (`self.PopulateBorder` (`self.Size`) (`self.BorderRooms`))
  (if (`self.ShowBorder`)
    (`/Game/Blueprints/Macros/BP_MyMacros.SpawnRooms` (`self.BorderRooms`) (`self.Size`) (`self.TileSize`) "/Game/Blueprints/Rooms/EndRooms/BP_EndRoom_00.BP_EndRoom_00_C"
      (:`Finished`
        _)))
  (`self.SetInitialRoom`)
  (while (`self.CurrentFreeSide`) :!label _label
    (`self.PickNearbyRoom`))
  (`KismetArrayLibrary.Array_Add` (`self.CheckedRooms`) (`self.CurrentRoom`))
  (`self.BackTrack`)
  (`/Game/Blueprints/Macros/BP_MyMacros.ConvertLastRoomBridge` (`self.BridgeRooms`) (`self.PathRooms`) (`self.CheckedRooms`) (`self.CurrentFreeSide`)
    (:`BridgesLeft`
      (goto _label))
    (:`NoBridgesLeft`
      (`/Game/Blueprints/Macros/BP_MyMacros.SpawnPathRooms` (`self.PathRooms`) (`self.Size`) (`self.TileSize`) "/Game/Blueprints/Rooms/BasicRooms/BP_BasicRoom_02.BP_BasicRoom_02_C"
        (:`Finished`
          (`self.PopulateWalls`)
          (if (`self.AllowLoopPaths`)
            (`self.AddLoopPaths`))
          (if (`self.ShowWalls`)
            (`/Game/Blueprints/Macros/BP_MyMacros.SpawnRooms` (`self.WallRooms`) (`self.Size`) (`self.TileSize`) "/Game/Blueprints/Rooms/StartRooms/BP_StartRoom_00.BP_StartRoom_00_C")))))))

(event `self.ReceiveTick`
  (params (DeltaSeconds :type "Float (single-precision)")))

(fn `AddBridgeAndPathRooms`
  (params (PathRoom :type Integer) (BridgeRoom :type Integer))
  (`KismetArrayLibrary.Array_Add` (`self.PathRooms`) PathRoom)
  (set `self.CurrentRoom` PathRoom)
  (`KismetArrayLibrary.Array_Add` (`self.BridgeRooms`) BridgeRoom))

(fn `AddLoopPaths`
  (locals (LoopPathsAdded :type Integer) (LoopPath :type Integer))
  (set `local.LoopPathsAdded` 0)
  (set `local.LoopPath` (`/Game/Blueprints/Macros/BP_MyMacros.GetRandomElement(Array)` (`self.WallRooms`) (`self.RandomStreamSeed`)) :!label _label)
  (if (`/Game/Blueprints/Macros/BP_MyMacros.RoomSurrounded` (`self.Size`) (`local.LoopPath`) (`self.PathRooms`))
    (if (< (`local.LoopPathsAdded`) (`self.MaxLoopPaths`))
      (goto _label))
    (else
      (`/Game/Blueprints/Macros/BP_MyMacros.AddAndRemoveItem(Array)` (`local.LoopPath`) (`self.PathRooms`) (`self.WallRooms`)
        (:`Out`
          (set `local.LoopPathsAdded` (+ (`local.LoopPathsAdded`) 1)))))))

(fn `BackTrack`
  (bind _arrayelement (`/Game/Blueprints/Macros/BP_MyMacros.ReverseForLoopWithBreak` (`self.PathRooms`) :!label _label)
    (:`LoopBody`
      (if (not (`KismetArrayLibrary.Array_Contains` (`self.CheckedRooms`) _arrayelement))
        (set `self.CurrentRoom` _arrayelement)
        (goto _label :!via `Break`)))))

(fn `PickNearbyRoom`
  (locals (CycleCounter :type Integer))
  (bind (_roominarray _pathroom _bridgeroom) (`/Game/Blueprints/Macros/BP_MyMacros.CheckNorthRoom` (`self.CurrentRoom`) (`self.Size`) false (`self.BorderRooms`) (`self.PathRooms`) (`self.BridgeRooms`)))
  (bind (_roominarray_2 _pathroom_2 _bridgeroom_2) (`/Game/Blueprints/Macros/BP_MyMacros.CheckNorthRoom` (`self.CurrentRoom`) (`self.Size`) true (`self.BorderRooms`) (`self.PathRooms`) (`self.BridgeRooms`)))
  (bind (_roominarray_3 _pathroom_3 _bridgeroom_3) (`/Game/Blueprints/Macros/BP_MyMacros.CheckEastRoom` (`self.CurrentRoom`) true (`self.BorderRooms`) (`self.PathRooms`) (`self.BridgeRooms`)))
  (bind (_roominarray_4 _pathroom_4 _bridgeroom_4) (`/Game/Blueprints/Macros/BP_MyMacros.CheckEastRoom` (`self.CurrentRoom`) false (`self.BorderRooms`) (`self.PathRooms`) (`self.BridgeRooms`)))
  (switch `int` (`KismetMathLibrary.RandomIntegerInRangeFromStream` 0 3 (`self.RandomStreamSeed`))
    (:`0`
      (if _roominarray :!label _label
        (`/Game/Blueprints/Macros/BP_MyMacros.CycleCounter` (`local.CycleCounter`) 4
          (:`True`
            (if _roominarray_2 :!label _label_2
              (`/Game/Blueprints/Macros/BP_MyMacros.CycleCounter` (`local.CycleCounter`) 4
                (:`True`
                  (if _roominarray_4 :!label _label_3
                    (`/Game/Blueprints/Macros/BP_MyMacros.CycleCounter` (`local.CycleCounter`) 4
                      (:`True`
                        (if _roominarray_3 :!label _label_4
                          (`/Game/Blueprints/Macros/BP_MyMacros.CycleCounter` (`local.CycleCounter`) 4
                            (:`True`
                              (goto _label))
                            (:`False`
                              (set `self.CurrentFreeSide` false :!label _label_5)))
                          (else
                            (`self.AddBridgeAndPathRooms` _pathroom_3 _bridgeroom_3))))
                      (:`False`
                        (goto _label_5)))
                    (else
                      (`self.AddBridgeAndPathRooms` _pathroom_4 _bridgeroom_4)
                      (goto _label_4))))
                (:`False`
                  (goto _label_5)))
              (else
                (`self.AddBridgeAndPathRooms` _pathroom_2 _bridgeroom_2))))
          (:`False`
            (goto _label_5)))
        (else
          (`self.AddBridgeAndPathRooms` _pathroom _bridgeroom))))
    (:`1`
      (goto _label_3))
    (:`2`
      (goto _label_2))
    (:`3`
      (goto _label_4)))
  (return))

(fn `PopulateBorder`
  (params (Size :type Integer) (BorderArray :type "Array of Integer"))
  (locals (L_Size :type Integer))
  (bind _l_size (`local.L_Size`))
  (bind _l_size_2 (`local.L_Size`))
  ;[1 1 1] North Border
  (set `local.L_Size` Size)
  (for _index (range (`local.L_Size`))
    (`KismetArrayLibrary.Array_Add` BorderArray _index))
  ;[1 1 1] East Border
  (for _index_2 (range 1 (+ (- (`local.L_Size`) 2) 1))
    (`KismetArrayLibrary.Array_Add` BorderArray (+ (* _index_2 _l_size_2) (- _l_size_2 1))))
  ;[1 1 1] South Border
  (for _index_3 (range 1 (+ (`local.L_Size`) 1))
    (`KismetArrayLibrary.Array_Add` BorderArray (+ (- _index_3 1) (* _l_size (- _l_size 1)))))
  ;[1 1 1] West Border
  (for _index_4 (range 1 (+ (- (`local.L_Size`) 2) 1))
    (`KismetArrayLibrary.Array_Add` BorderArray (* _index_4 (`local.L_Size`)))))

(fn `PopulateFakeBorder`
  (params (Size :type Integer) (BorderArray :type "Array of Integer"))
  (locals (L_Size :type Integer))
  (bind _l_size (`local.L_Size`))
  (bind _l_size_2 (`local.L_Size`))
  ;[1 1 1] North Border
  (set `local.L_Size` Size)
  (for _index (range (`local.L_Size`))
    (`KismetArrayLibrary.Array_Add` BorderArray _index))
  ;[1 1 1] East Border
  (for _index_2 (range 1 (+ (- (`local.L_Size`) 2) 1))
    (`KismetArrayLibrary.Array_Add` BorderArray (+ (* _index_2 _l_size_2) (- _l_size_2 1))))
  ;[1 1 1] South Border
  (for _index_3 (range 1 (+ (`local.L_Size`) 1))
    (`KismetArrayLibrary.Array_Add` BorderArray (+ (- _index_3 1) (* _l_size (- _l_size 1)))))
  ;[1 1 1] West Border
  (for _index_4 (range 1 (+ (- (`local.L_Size`) 2) 1))
    (`KismetArrayLibrary.Array_Add` BorderArray (* _index_4 (`local.L_Size`)))))

(fn `PopulateWalls`
  (bind _size (`self.Size`))
  (for _index (range (* _size _size))
    (if (not (`/Game/Blueprints/Macros/BP_MyMacros.CheckRoomArrays` _index (`self.BorderRooms`) (`self.PathRooms`) (`self.BridgeRooms`)))
      (`KismetArrayLibrary.Array_Add` (`self.WallRooms`) _index))))

(fn `SetInitialRoom`
  (locals (FakeInnerBorder :type "Array of Integer"))
  (set `self.CurrentRoom` (+ (`self.Size`) 1))
  (`KismetArrayLibrary.Array_Add` (`self.PathRooms`) (`self.CurrentRoom`)))

(fn `UserConstructionScript`)