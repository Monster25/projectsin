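; BP_Enemy is an enemy actor that takes damage and drops a random item when it dies.
; DealDamageToMe subtracts incoming damage from Health, then calls SpawnItem and destroys the actor once Health reaches zero.
; SpawnItem spawns an ItemSpawnClass actor at its location, picks a random LootTable row, follows that row's item handle into the item table and passes the ID via SetItemId.
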(fn `DealDamageToMe`
  (params (IncomingDamage :type "Float (double-precision) (by ref)"))
  (bind _health (`self.Health`))
  (set `self.Health` (- _health IncomingDamage))
  (if (<= _health 0.0)
    (`self.SpawnItem`)
    (`self.K2_DestroyActor`)))

(fn `SpawnItem`
  (bind _outrownames (`DataTableFunctionLibrary.GetDataTableRowNames` (`self.LootTable`)))
  (bind _result (`/Engine/EditorBlueprintResources/StandardMacros.DecrementInt` (`KismetArrayLibrary.Array_Length` _outrownames))
    (:`  `
      (bind _returnvalue (`|SpawnActorFromClass` (`self.ItemSpawnClass`) (`KismetMathLibrary.Conv_VectorToTransform` (`self.K2_GetActorLocation`)) "Undefined" "OverrideRootScale" null null))
      (bind _returnvalue_2 (`|GetDataTableRow` (`self.LootTable`) (`|GetArrayItem` _outrownames (`KismetMathLibrary.RandomIntegerInRange` 0 _result)))
        (:`then`
          (bind (_datatable _rowname) (break `DataTableRowHandle` (`.ItemRef_2_29F2FD6546C5CB6F6622CE8DA0C13A1D` (break `/Game/Blueprints/GameData/Items/Structures/Struct_LootTableData` _returnvalue_2))))
          (bind _returnvalue_3 (`|GetDataTableRow` _datatable _rowname)
            (:`then`
              (`/Game/Blueprints/Pickups/BP_Item.SetItemId` _returnvalue (`.ID_11_05CB8AEF472481D61C5566A382762853` (break `/Game/Blueprints/GameData/Items/Structures/Struct_EquipmentData` _returnvalue_3))))))))))

(fn `UserConstructionScript`)