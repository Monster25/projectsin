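; Debug actor that shows the frame rate and the player character's state on screen.
; On BeginPlay it runs the stat FPS console command and adds a GUI_Debug widget to the viewport.
; Every Tick it polls PlayerChar for the current and previous player state enums and writes them as labeled text into the widget.
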(event `self.ReceiveBeginPlay`
  (`KismetSystemLibrary.ExecuteConsoleCommand` "stat FPS" null)
  (bind _returnvalue (`|CreateWidget` "/Game/Blueprints/GUI/GUI_Debug.GUI_Debug_C" (`GameplayStatics.GetPlayerController` 0)))
  (`UserWidget.AddToViewport` _returnvalue 0))

(event `self.ReceiveTick`
  (params (DeltaSeconds :type "Float (single-precision)"))
  (bind _playerchar (`self.PlayerChar`))
  (`|ExecutionSequence`
    (:`then_0`
      (bind _state (`/Game/Blueprints/Player/MyCharacter.GetCurrentPlayerState` _playerchar))
      (`TextBlock.SetText` (`/Game/Blueprints/GUI/GUI_Debug.PlayerState` (stale `self.ReceiveBeginPlay` _returnvalue)) (`KismetTextLibrary.Conv_StringToText` (`KismetStringLibrary.Concat_StrStr` "Current Player State: " (`|GetEnumeratorNameAsString` _state)))))
    (:`then_1`
      (bind _state_2 (`/Game/Blueprints/Player/MyCharacter.GetPreviousPlayerState` _playerchar))
      (`TextBlock.SetText` (`/Game/Blueprints/GUI/GUI_Debug.PlayerPreviousState` (stale `self.ReceiveBeginPlay` _returnvalue)) (`KismetTextLibrary.Conv_StringToText` (`KismetStringLibrary.Concat_StrStr` "Previous Player State: " (`|GetEnumeratorNameAsString` _state_2)))))))

(fn `UserConstructionScript`)