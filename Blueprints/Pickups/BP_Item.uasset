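; BP_Item is a world pickup that adds its item ID to the player's inventory on touch.
; A box overlap casts the other actor to MyCharacter and calls PickupItem, which checks for an InventoryComponent.
; If present, it adds the item, prints the item's information from that component and destroys itself.
; Setter and getter functions expose the ItemId.
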(event `self.ReceiveBeginPlay`)

(event `self.Box.OnComponentBeginOverlap`
  (params (OverlappedComponent :type "PrimitiveComponent Object Reference") (OtherActor :type "Actor Object Reference") (OtherComp :type "PrimitiveComponent Object Reference") (OtherBodyIndex :type Integer) (bFromSweep :type Boolean) (SweepResult :type "HitResult Structure (by ref)"))
  (bind _asmy_character (cast `/Game/Blueprints/Player/MyCharacter` OtherActor))
  (`self.PickupItem` _asmy_character))

(fn `GetItemId`
  (returns (Value :type Integer))
  (return (`self.ItemId`)))

(fn `PickupItem`
  (params (OverlappedActor :type "/Game/Blueprints/Player/MyCharacter Object Reference (by ref)"))
  (bind _itemid (`self.ItemId`))
  (bind _value (`/Game/Blueprints/Player/MyCharacter.ComponentChecker` OverlappedActor "/Game/Blueprints/GameLogic/InventoryComponent.InventoryComponent_C"))
  (if _value
    (bind _inventorycomponent (`/Game/Blueprints/Player/MyCharacter.GetInventoryComponent` OverlappedActor))
    (`/Game/Blueprints/GameLogic/InventoryComponent.AddItem` _inventorycomponent _itemid)
    (bind _information (`/Game/Blueprints/GameLogic/InventoryComponent.GetItemInformation` _inventorycomponent _itemid))
    (`KismetSystemLibrary.PrintString` _information)
    (`self.K2_DestroyActor`)))

(fn `SetItemId`
  (params (ItemId :type "Integer (by ref)"))
  (set `self.ItemId` ItemId))

(fn `UserConstructionScript`)